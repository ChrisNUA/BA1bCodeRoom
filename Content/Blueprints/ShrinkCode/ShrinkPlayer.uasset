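; ShrinkPlayer is a trigger that temporarily shrinks the third-person player character when it overlaps the box.
; BeginPlay caches the player as BP_ThirdPersonCharacter, and the box overlap reacts only to that character.
; On overlap it sets the character's BeenShrunkPreviously flag, scales the actor down through SetScaleSmall, then restores normal scale through SetScaleNormal after a short Delay.
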(event `self.ReceiveBeginPlay`
  (bind _asbp_third_person_character (cast `/Game/ThirdPerson/Blueprints/BP_ThirdPersonCharacter` (`GameplayStatics.GetPlayerCharacter` 0)))
  (set `self.As BP Third Person Character` _asbp_third_person_character))

(event `self.BoxOverlap.OnComponentBeginOverlap`
  (params (OverlappedComponent :type "PrimitiveComponent Object Reference") (OtherActor :type "Actor Object Reference") (OtherComp :type "PrimitiveComponent Object Reference") (OtherBodyIndex :type Integer) (bFromSweep :type Boolean) (SweepResult :type "HitResult Structure (by ref)"))
  (bind _as_bp_third_person_character (`self.As BP Third Person Character`))
  ;[1 1 1] If the character overlaps the box. True/False
  (if (== OtherActor _as_bp_third_person_character)
    (set `/Game/ThirdPerson/Blueprints/BP_ThirdPersonCharacter.BeenShrunkPreviously` true _as_bp_third_person_character)
    ;[1 1 1] If true, set scale to small using functions. Double click functions on the left to see code.
    (`self.SetScaleSmall`)
    (`KismetSystemLibrary.Delay` 3.0)
    (`self.SetScaleNormal`)))

(fn `SetScaleNormal`
  ;[1 1 1] Set character scale to 1
  (`self.SetActorScale3D` (`self.As BP Third Person Character`) (1.0 1.0 1.0)))

(fn `SetScaleSmall`
  ;[1 1 1] Set character scale to 0.4
  (`self.SetActorScale3D` (`self.As BP Third Person Character`) (0.4 0.4 0.4)))

(fn `UserConstructionScript`)