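; BP_RestrictCamera is a trigger volume that puts the third-person character into platformer mode while inside it.
; On BeginPlay it caches the player character and copies its Arrow's world rotation into the character's WorldRotationForCamera.
; Box overlap begin sets the character's PlatformerMode flag; overlap end clears it and calls ResetDoOnce so the camera can reset again.
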(event `self.ReceiveBeginPlay`
  ;[1 1 1] Get info for third person character. Set world rotation to reset camera based on the big red arrow.
  (bind _asbp_third_person_character (cast `/Game/ThirdPerson/Blueprints/BP_ThirdPersonCharacter` (`GameplayStatics.GetPlayerCharacter` 0)))
  (bind _output_get (set `self.As BP Third Person Character` _asbp_third_person_character))
  (set `/Game/ThirdPerson/Blueprints/BP_ThirdPersonCharacter.WorldRotationForCamera` (`SceneComponent.K2_GetComponentRotation` (`self.Arrow`)) _output_get))

(event `self.Box.OnComponentBeginOverlap`
  (params (OverlappedComponent :type "PrimitiveComponent Object Reference") (OtherActor :type "Actor Object Reference") (OtherComp :type "PrimitiveComponent Object Reference") (OtherBodyIndex :type Integer) (bFromSweep :type Boolean) (SweepResult :type "HitResult Structure (by ref)"))
  ;[1 1 1] Switches to platformer mode, Boolean is held inside 3rd person character
  (if (== (`self.As BP Third Person Character`) OtherActor)
    (set `/Game/ThirdPerson/Blueprints/BP_ThirdPersonCharacter.PlatformerMode` true (`self.As BP Third Person Character`))))

(event `self.Box.OnComponentEndOverlap`
  (params (OverlappedComponent :type "PrimitiveComponent Object Reference") (OtherActor :type "Actor Object Reference") (OtherComp :type "PrimitiveComponent Object Reference") (OtherBodyIndex :type Integer))
  (bind _as_bp_third_person_character (`self.As BP Third Person Character`))
  ;[1 1 1] Switches back out of platformer mode and resets the do once so we can reset camera again.
  (if (== (`self.As BP Third Person Character`) OtherActor)
    (set `/Game/ThirdPerson/Blueprints/BP_ThirdPersonCharacter.PlatformerMode` false _as_bp_third_person_character)
    (`/Game/ThirdPerson/Blueprints/BP_ThirdPersonCharacter.ResetDoOnce` _as_bp_third_person_character)))

(fn `UserConstructionScript`)