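; A jump pad that launches the third-person player character into the air, but only while the character is shrunk.
; On BeginPlay it caches the player character, then a box overlap checks that the overlapping actor is that character and that its IsSmall flag is set.
; The launch overrides vertical velocity with the character's jump Z velocity scaled by the Jumpheight multiplier, which controls pad strength.
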(event `self.ReceiveBeginPlay`
  ;[1 1 1] Store third person character for later use.
  (bind _asbp_third_person_character (cast `/Game/ThirdPerson/Blueprints/BP_ThirdPersonCharacter` (`GameplayStatics.GetPlayerCharacter` 0)))
  (set `self.As BP Third Person Character` _asbp_third_person_character))

(event `self.Box.OnComponentBeginOverlap`
  (params (OverlappedComponent :type "PrimitiveComponent Object Reference") (OtherActor :type "Actor Object Reference") (OtherComp :type "PrimitiveComponent Object Reference") (OtherBodyIndex :type Integer) (bFromSweep :type Boolean) (SweepResult :type "HitResult Structure (by ref)"))
  (bind _as_bp_third_person_character (`self.As BP Third Person Character`))
  ;[1 1 1] If the character overlaps the jump pad > Launch
  (if (and (== OtherActor _as_bp_third_person_character) (`/Game/ThirdPerson/Blueprints/BP_ThirdPersonCharacter.IsSmall` _as_bp_third_person_character))
    ;[1 1 1] Launcher the character into the air using the Jump Z velocity. You can edit strength of jumpPad through the multiplication value.
    (`Character.LaunchCharacter` _as_bp_third_person_character (`KismetMathLibrary.MakeVector` 0.0 0.0 (* (`CharacterMovementComponent.JumpZVelocity` (`Character.CharacterMovement` _as_bp_third_person_character)) (`self.Jumpheight`))) false true)))

(fn `UserConstructionScript`)