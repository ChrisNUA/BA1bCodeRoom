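; Collectible coin Blueprint that the third-person player character picks up by walking into its overlap sphere.
; BeginPlay caches the player character, and a sphere overlap with that character destroys the coin and passes its CoinValue to the character's CoinCounter.
; CoinValue is intended to be set in the editor, so coins can differ in worth.
; The construction script randomizes the RotatingMovement rate so coins spin at varied speeds.
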(event `self.ReceiveBeginPlay`
  ;[1 1 1] Store third person variable for later use.
  (bind _asbp_third_person_character (cast `/Game/ThirdPerson/Blueprints/BP_ThirdPersonCharacter` (`GameplayStatics.GetPlayerCharacter` 0)))
  (set `self.As BP Third Person Character` _asbp_third_person_character))

(event `self.SphereOverlap.OnComponentBeginOverlap`
  (params (OverlappedComponent :type "PrimitiveComponent Object Reference") (OtherActor :type "Actor Object Reference") (OtherComp :type "PrimitiveComponent Object Reference") (OtherBodyIndex :type Integer) (bFromSweep :type Boolean) (SweepResult :type "HitResult Structure (by ref)"))
  (bind _as_bp_third_person_character (`self.As BP Third Person Character`))
  ;[1 1 1] Check whether the third person
  (if (== OtherActor _as_bp_third_person_character)
    ;[1 1 1] Destroy the instance of the coin within the game world.
    (`self.K2_DestroyActor`)
    ;[1 1 1] Fire off the coin counter function within the third person character. Utilising the coin value to change the value of each coin depending on size, placement etc. This makes coins very dynamic as we can set the value in the unreal editor.
    (`/Game/ThirdPerson/Blueprints/BP_ThirdPersonCharacter.CoinCounter` _as_bp_third_person_character (`self.CoinValue`))))

(fn `UserConstructionScript`
  (set `RotatingMovementComponent.RotationRate` (`KismetMathLibrary.MakeRotator` 0.0 0.0 (`KismetMathLibrary.RandomFloatInRange` 100.0 250.0)) (`self.RotatingMovement`)))