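; Bomb actor that explodes on a short fuse and notifies any AI pigs caught in its kill radius.
; BeginPlay gives the Bomb component a random spin so it rolls on landing.
; The BombExplosion event uses actor life span as the fuse and binds TriggerExplosion to OnDestroyed.
; TriggerExplosion spawns the explosion particles and sends an InteractWith interface message to each BP_AIPig overlapping KillRadius.
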(event `self.ReceiveBeginPlay`
  ;[1 1 1] Gets the bomb rolling as soon as it hits the ground.
  (`PrimitiveComponent.SetPhysicsAngularVelocityInDegrees` (`self.Bomb`) (* (`KismetMathLibrary.RandomUnitVector`) 10.0) false "None"))

(event `BombExplosion`
  ;[0.6493 1 0.2389] BombExplosionLogic
  ;;[1 1 1] We don't want loads of bombs in our map. You can set the life span to whatever number you wish.
  (`self.SetLifeSpan` self 3.0)
  ;;[1 1 1] Once the life span runs out we want to fire off an explosion and check if pigs are in radius of explosion. We can do this by overriding the 'on destroyed event.
  (add `self.OnDestroyed` self (delegate `Trigger Explosion`)))

(event `Trigger Explosion` :!signature `self.OnDestroyed`
  (params (DestroyedActor :type "Actor Object Reference"))
  ;[0.6493 1 0.2389] BombExplosionLogic
  ;;[1 1 1] Visuals for the explosion.
  (`GameplayStatics.SpawnEmitterAtLocation` "/Game/StarterContent/Particles/P_Explosion.P_Explosion" (`self.K2_GetActorLocation` DestroyedActor))
  ;;[1 1 1] Checks the overlapping actors against our kill radius.
  (for _array_element (`PrimitiveComponent.GetOverlappingActors` (`self.KillRadius`) "/Game/Blueprints/FarmCode/PigCode/BP_AIPig.BP_AIPig_C")
    ;;[1 1 1] Fire of our blueprint interface which is picked up in BP_AiPig (Only called if in radius)
    (message `/Game/Blueprints/Interfaces/BPI_Trigger.InteractWith` _array_element)))

(fn `UserConstructionScript`)