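; BP_AIPig is a farm pig that wanders, grows when fed and can be killed by a bomb for harvesting.
; A looping timer drives random navmesh moves with grunts, while food events scale up the body.
; On a hit, it stops moving, snaps the body to the floor via line trace, tips it over with a timeline, squeals and reveals harvest text.
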(event `NoticeFood`
  (params (PigFood :type "StaticMeshComponent Object Reference"))
  (bind _pigbody (`self.PigBody`))
  (`SceneComponent.SetRelativeScale3D` _pigbody (+ (`self.AddScale`) (`SceneComponent.RelativeScale3D` _pigbody))))

(event `self.ReceiveBeginPlay`
  ;[1 1 1] Start a looping event so the pig is always moving. Until its hit by below code.
  (bind _returnvalue (`KismetSystemLibrary.K2_SetTimerDelegate` (delegate `AiMove`) (`self.MovementTime`) true))
  (set `self.AiMoveTimerHandle` _returnvalue))

(event `AiMove`
  ;[1 1 1] Gets a random point within the 'Nav Mesh Bounds'. Press P to see the nav mesh in the game editor. This makes the pig move randomly.
  (`|AIMoveTo` self (`NavigationSystemV1.K2_GetRandomReachablePointInRadius` (`self.K2_GetActorLocation`) 2000.0 null null) null 50.0
    (:`then`
      ;[1 1 1] Plays a random grunt when moving
      (`GameplayStatics.PlaySoundAtLocation` "/Game/Blueprints/FarmCode/PigCode/MS_Grunt.MS_Grunt" (`self.K2_GetActorLocation`) (struct) 1.0 1.0 0.0 "/Game/Blueprints/FarmCode/PigCode/NewSoundAttenuation.NewSoundAttenuation" null null null))))

(event `/Game/Blueprints/Interfaces/BPI_Trigger.InteractWith`
  (bind _pigbody (`self.PigBody`))
  (bind _returnvalue (`SceneComponent.K2_GetComponentLocation` _pigbody))
  ;[1 1 1] Only fires off when the bomb hits the pig.
  (if (not (`self.IsDead`))
    ;[1 1 1] Reveal harvest text to show you can use E to farm.
    (`SceneComponent.SetHiddenInGame` (`self.HarvestText`) false false)
    ;[1 1 1] Immediately stop the character movement so we get no sliding effects.
    (`MovementComponent.StopMovementImmediately` (`self.CharacterMovement`))
    ;[1 1 1] Stops the movement loop.
    (`KismetSystemLibrary.K2_ClearAndInvalidateTimerHandle` (`self.AiMoveTimerHandle`))
    (bind _outhit (`KismetSystemLibrary.LineTraceSingle` _returnvalue (+ _returnvalue (* (`SceneComponent.GetUpVector` _pigbody) (`self.TraceDistance`))) "TraceTypeQuery1"))
    ;[1 1 1] Sets the world location of the pig body using the impact point.
    (`SceneComponent.K2_SetWorldLocation` (`self.PigBody`) (+ (`.ImpactPoint` (`GameplayStatics.BreakHitResult` _outhit)) (0.0 0.0 20.0)) false false)
    ;[1 1 1] A quick way of 'animating' a death. Double click to open chart.
    (bind (_direction _animatetrack) (`Timeline|DeathAnimate`)
      (:`Update`
        ;[1 1 1] Rotates the pig 90 degrees on the X axis over the period of time specified within the timeline (0.5 seconds)
        (`SceneComponent.K2_SetRelativeRotation` (`self.PigBody`) (`KismetMathLibrary.MakeRotator` (`KismetMathLibrary.Lerp` 0.0 90.0 _animatetrack)) false false)
        (set `self.IsDead` true)
        ;[1 1 1] Play Squeal upon death. Do once as the bomb rolls and may trigger hit too many times.
        (`/Engine/EditorBlueprintResources/StandardMacros.DoOnce` false
          (:`Completed`
            (`GameplayStatics.PlaySoundAtLocation` "/Game/Blueprints/FarmCode/PigCode/MS_Squeal.MS_Squeal" (`self.K2_GetActorLocation`) (struct) 1.0 1.0 0.0 null null null null)))))))

(event `/Game/Blueprints/Interfaces/BPI_Trigger.SpottedFood`
  ;[1 1 1] Check if the pig is dead
  (if (not (`self.IsDead`))
    ;[1 1 1] Upscale the pig!
    (`SceneComponent.SetRelativeScale3D` (`self.PigBody`) (`KismetMathLibrary.ClampVectorSize` (+ (`SceneComponent.K2_GetComponentScale` (`self.PigBody`)) (0.2 0.2 0.2)) 1.0 2.0))))

(fn `UserConstructionScript`)