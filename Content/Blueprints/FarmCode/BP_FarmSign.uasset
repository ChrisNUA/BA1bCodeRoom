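; Farm sign actor that drops temporary objects, commented as food, when the player walks into its trigger box.
; BeginPlay caches the player's third-person character, and the box overlap responds only to that actor.
; Each overlap loops on a configurable amount, spawning the chosen class at the SpawnPoint actor's transform with a set life span.
; The construction script writes the editable text value to the sign's TextRender.
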(event `self.ReceiveBeginPlay`
  ;[1 1 1] Soft cast to player character
  (bind _asbp_third_person_character (cast `/Game/ThirdPerson/Blueprints/BP_ThirdPersonCharacter` (`GameplayStatics.GetPlayerCharacter` 0)))
  (set `self.As BP Third Person Character` _asbp_third_person_character))

(event `self.Box.OnComponentBeginOverlap`
  (params (OverlappedComponent :type "PrimitiveComponent Object Reference") (OtherActor :type "Actor Object Reference") (OtherComp :type "PrimitiveComponent Object Reference") (OtherBodyIndex :type Integer) (bFromSweep :type Boolean) (SweepResult :type "HitResult Structure (by ref)"))
  (bind _spawnpoint (`self.SpawnPoint`))
  ;[1 1 1] Once the character overlaps this box. Trigger the concurrent nodes
  (if (== OtherActor (`self.As BP Third Person Character`))
    ;[1 1 1] Spawn 5 balls of food. You can edit the amount of food in 'Amount Spawned' variable
    (for _ (range (+ (`self.AmountSpawned`) 1))
      ;[1 1 1] Spawns whatever actor you place into 'Object to spawn'
      (`/Engine/EditorBlueprintResources/StandardMacros.IsValid` _spawnpoint
        (:`Is Valid`
          (bind _returnvalue (`|SpawnActorFromClass` (`self.ObjectToSpawn`) (`self.GetTransform` _spawnpoint) "Undefined" "MultiplyWithRoot" null null))
          ;[1 1 1] Sets life spawn to whatever you place into 'Life span time'
          (`self.SetLifeSpan` _returnvalue (`self.LifeSpanTime`)))))))

(fn `UserConstructionScript`
  (`TextRenderComponent.K2_SetText` (`self.TextRender`) (`self.TextValue`)))