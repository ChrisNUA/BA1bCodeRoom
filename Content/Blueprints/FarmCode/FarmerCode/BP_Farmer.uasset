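; Farmer NPC with a looping or timed head-bob animation that shows dialogue to the player through a narrative widget.
; A trigger box sets an overlap flag when the player enters.
; Each Interactwith event advances through the Dialogue array, reusing one WBP_FarmerDialogue widget.
; Passing the last line or the player leaving the box removes the widget, clears its reference and resets the index.
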(event `self.ReceiveBeginPlay`
  ;[1 1 1] Stores our cast into a variable for later use
  (bind _asbp_third_person_character (cast `/Game/ThirdPerson/Blueprints/BP_ThirdPersonCharacter` (`GameplayStatics.GetPlayerCharacter` 0)))
  (set `self.As BP Third Person Character` _asbp_third_person_character)
  ;[1 1 1] Creating a bobbing head motion
  (bind (_direction _bobbingheadtrack) (`Timeline|BobbingHead`)
    (:`Update`
      (`SceneComponent.K2_SetRelativeLocation` (`self.Farmer`) (`KismetMathLibrary.MakeVector` 0.0 0.0 (`KismetMathLibrary.Lerp` 0.0 15.0 _bobbingheadtrack)) false false))))

(event `self.TriggerBoxx.OnComponentBeginOverlap`
  (params (OverlappedComponent :type "PrimitiveComponent Object Reference") (OtherActor :type "Actor Object Reference") (OtherComp :type "PrimitiveComponent Object Reference") (OtherBodyIndex :type Integer) (bFromSweep :type Boolean) (SweepResult :type "HitResult Structure (by ref)"))
  ;[1 1 1] When the third person overlaps the box trigger we set a variable to true. Otherwise the character could trigger the dialogue outside of box range
  (if (== (`self.As BP Third Person Character`) OtherActor)
    (set `self.OverlappingBox` true)))

(event `/Game/Blueprints/Interfaces/BPI_Trigger.InteractWith`
  ;[1 1 1] Only triggered when the player walks into the box and presses E
  ;[1 1 1] Checks to see if we've worked through our dialogue. Length is excellent because if we add more dialogue later down the line it will adapt dynamically
  (`/Engine/EditorBlueprintResources/StandardMacros.IncrementInt` (`self.DialogueIndex`)
    (:`  `
      (if (< (`self.DialogueIndex`) (`KismetArrayLibrary.Array_Length` (`self.Dialogue`)))
        ;[1 1 1] This is here to prevent multiple widgets being placed on our screen.
        (`self.NarrativeWidget`
          (:`then`
            _)
          (:`else`
            ;[1 1 1] Create our widget, store into a variable and display on players screen
            (bind _returnvalue (`|CreateWidget` "/Game/Blueprints/FarmCode/FarmerCode/WBP_FarmerDialogue.WBP_FarmerDialogue_C"))
            (bind _output_get (set `self.NarrativeWidget` _returnvalue))
            (`UserWidget.AddToViewport` _output_get 0)))
        ;[1 1 1] Sets the phrarses we've made inside Dialogue and places them into our user interface widget. See WBP_FarmerDialogue for more info
        (`TextBlock.SetText` (`/Game/Blueprints/FarmCode/FarmerCode/WBP_FarmerDialogue.Narrative` (`self.NarrativeWidget`)) (`KismetTextLibrary.Conv_StringToText` (`|GetArrayItem` (`self.Dialogue`) (`self.DialogueIndex`))))
        (else
          ;[1 1 1] Remove widget from screen. Set the widget back to blank otherwise the validated GET above this code would get confused. Sets dialogue index back to -1 (arrays always start at 0)
          (`Widget.RemoveFromParent` (`self.NarrativeWidget`) :!label _label)
          (set `self.NarrativeWidget` null)
          (set `self.DialogueIndex` -1))))))

(event `self.TriggerBoxx.OnComponentEndOverlap`
  (params (OverlappedComponent :type "PrimitiveComponent Object Reference") (OtherActor :type "Actor Object Reference") (OtherComp :type "PrimitiveComponent Object Reference") (OtherBodyIndex :type Integer))
  ;[1 1 1] If we walk out of the triggerbox, change the overlapping variable accordingly.
  (set `self.OverlappingBox` false)
  ;[1 1 1] Double checking its the player that caused this overlap. Could be a rogue pig walking by!
  (if (== OtherActor (`self.As BP Third Person Character`))
    ;[1 1 1] Prevents bugs and makes sure the narrative widget doesn't execute if it contains 'none'
    (`/Engine/EditorBlueprintResources/StandardMacros.IsValid` (`self.NarrativeWidget`)
      (:`Is Valid`
        (goto _label)))))

(fn `UserConstructionScript`)