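; Farm sign trap that spawns a bomb when the player walks into its trigger box.
; BeginPlay caches the player's third-person character, which the overlap check compares against before spawning BP_Bomb at the SpawnPoint location and calling BombExplosion on it.
; A local BombExplosion event spawns the explosion particle effect at a destroyed actor's location, with no binding to it shown.
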(event `self.ReceiveBeginPlay`
  (bind _asbp_third_person_character (cast `/Game/ThirdPerson/Blueprints/BP_ThirdPersonCharacter` (`GameplayStatics.GetPlayerCharacter` 0)))
  (set `self.As BP Third Person Character` _asbp_third_person_character))

(event `self.TriggerBox.OnComponentBeginOverlap`
  (params (OverlappedComponent :type "PrimitiveComponent Object Reference") (OtherActor :type "Actor Object Reference") (OtherComp :type "PrimitiveComponent Object Reference") (OtherBodyIndex :type Integer) (bFromSweep :type Boolean) (SweepResult :type "HitResult Structure (by ref)"))
  ;[1 1 1] Once the player walks through the triggerbox > spawn the bomb at the targetpoint location
  (if (== (`self.As BP Third Person Character`) OtherActor)
    (bind _returnvalue (`|SpawnActorFromClass` "/Game/Blueprints/FarmCode/BP_Bomb.BP_Bomb_C" (`KismetMathLibrary.MakeTransform` (`self.K2_GetActorLocation` (`self.SpawnPoint`))) "Undefined" "MultiplyWithRoot" null null))
    (`/Game/Blueprints/FarmCode/BP_Bomb.BombExplosion` _returnvalue)))

(event `BombExplosion`
  (params (DestroyedActor :type "Actor Object Reference"))
  ;[1 1 1] Visuals for the explosion.
  (`GameplayStatics.SpawnEmitterAtLocation` "/Game/StarterContent/Particles/P_Explosion.P_Explosion" (`self.K2_GetActorLocation` DestroyedActor)))

(fn `UserConstructionScript`)